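; Main menu actor that spawns the WBP_MainMenu widget on BeginPlay and handles its input focus.
; Non-mouse key presses move keyboard focus to the mouse sensitivity option or the Start Game button, depending on the visible panel.
; Gamepad face-button-right backs out of Options to the main menu.
; Left click returns focus to the game viewport and shows the cursor.
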(event EventBeginPlay
  (bind _returnvalue (UserInterface|CreateWidget "/Game/UI/WBP_MainMenu.WBP_MainMenu_C" (Game|GetPlayerController 0)))
  (bind _output_get (Variables|Default|SetMainMenu _returnvalue))
  (UserInterface|Viewport|AddtoViewport _output_get 0))

(event Collision|EventActorBeginOverlap
  (params (OtherActor :type Actor%20Object%20Reference)))

(event EventTick
  (params (DeltaSeconds :type Float%20%28single-precision%29)))

(event Input|KeyboardEvents|AnyKey
  (params (Key :type Key%20Structure :default "None"))
  (bind _mainmenu (Variables|Default|GetMainMenu))
  (:Pressed
    (if (not (Class|KismetInputLibrary|KeyIsMouseButton Key))
      (if (Widget|IsVisible (Variables|/Game/UI/WBP_MainMenu.WBP_MainMenu_C|GetOptionsVb _mainmenu))
        (Widget|SetKeyboardFocus (Variables|/Game/UI/WBP_MainMenu.WBP_MainMenu_C|GetMouseSensitivity _mainmenu))
        (elif (Widget|IsVisible _mainmenu)
          (Widget|SetKeyboardFocus (Variables|/Game/UI/WBP_MainMenu.WBP_MainMenu_C|GetStartGameButton _mainmenu)))))))

(event Input|GamepadEvents|GamepadFaceButtonRight
  (params (Key :type Key%20Structure :default "None"))
  (bind _mainmenu (Variables|Default|GetMainMenu))
  (:Pressed
    (if (Widget|IsVisible (Variables|/Game/UI/WBP_MainMenu.WBP_MainMenu_C|GetOptionsVb _mainmenu))
      (Default|OptionstoMain _mainmenu))))

(event Input|MouseEvents|LeftMouseButton
  (params (Key :type Key%20Structure :default "None"))
  (:Pressed
    (Class|WidgetBlueprintLibrary|SetFocustoGameViewport)
    (Variables|/Script/Engine.PlayerController|SetbShowMouseCursor (Game|GetPlayerController 0) true)))

(fn ConstructionScript)