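; Player shooter character Blueprint that handles HUD display, an intro sound and the pause menu.
; BeginPlay shows the controller's HUD and creates a collapsed pause widget.
; Escape, P and gamepad Start share a FlipFlop that toggles pause, input mode and cursor, saving mouse and gamepad sensitivities on resume.
; Other input handlers back out of options, restore menu focus for non-mouse navigation, and return focus to the viewport on left click.
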(event EventBeginPlay
  (|CallParentFunction)
  (Variables|/Script/Engine.PlayerController|SetbShowMouseCursor (Game|GetPlayerController 0) false)
  (bind _asshooter_player_controller (Utilities|Casting|CastToShooterPlayerController (Game|GetPlayerController 0)))
  (bind _output_get (Variables|Default|SetHUD (Variables|/Script/SimpleShooter.ShooterPlayerController|GetHUD _asshooter_player_controller)))
  (Widget|SetVisibility _output_get "Visible")
  (bind _returnvalue (UserInterface|CreateWidget "/Game/UI/WBP_PauseMenu1.WBP_PauseMenu1_C" (Game|GetPlayerController 0)))
  (bind _output_get_2 (Variables|Default|SetPause%20Menu%20Widget _returnvalue))
  (UserInterface|Viewport|AddtoViewport _output_get_2 0)
  (Widget|SetVisibility _output_get_2 "Collapsed")
  (Audio|PlaySoundatLocation "/Game/AssetPacks/GameDevTV/VoiceOvers/Intro.Intro" (Transformation|GetActorLocation (Game|Player|GetPlayerPawn 0)) "0, 0, 0" 1.0 1.0 0.0 0 0 0))

(event Collision|EventActorBeginOverlap
  (params (OtherActor :type Actor%20Object%20Reference))
  (|CallParentFunction OtherActor))

(event EventTick
  (params (DeltaSeconds :type Float%20%28single-precision%29))
  (|CallParentFunction DeltaSeconds))

(event Input|GamepadEvents|GamepadSpecialRight
  (params (Key :type Key%20Structure :default "None"))
  (bind _pause_menu_widget (Variables|Default|GetPause%20Menu%20Widget))
  (bind _pause_menu_widget_2 (Variables|Default|GetPause%20Menu%20Widget))
  (bind _pause_menu_widget_3 (Variables|Default|GetPause%20Menu%20Widget))
  (:Pressed
    (Utilities|FlowControl|FlipFlop
      (:A
        (Game|SetGamePaused true)
        (Input|SetInputModeGameandUI (Game|GetPlayerController 0) (Variables|Default|GetPause%20Menu%20Widget) "DoNotLock" true)
        (Widget|SetVisibility _pause_menu_widget_3 "Visible")
        (Widget|SetVisibility (Variables|/Game/UI/WBP_PauseMenu1.WBP_PauseMenu1_C|GetMainMenuButtonsVB _pause_menu_widget_3) "Visible")
        (Widget|SetVisibility (Variables|/Game/UI/WBP_PauseMenu1.WBP_PauseMenu1_C|GetMainMenuAllVB _pause_menu_widget_3) "Visible")
        (Variables|/Script/Engine.PlayerController|SetbShowMouseCursor (Game|GetPlayerController 0) true))
      (:B
        (Game|SetGamePaused false)
        (Input|SetInputModeGameOnly (Game|GetPlayerController 0))
        (Widget|SetVisibility _pause_menu_widget_3 "Collapsed")
        (Variables|/Script/Engine.PlayerController|SetbShowMouseCursor (Game|GetPlayerController 0) false)
        (Default|SaveGame _pause_menu_widget (Class|Slider|GetValue (Variables|/Game/UI/WBP_PauseMenu1.WBP_PauseMenu1_C|GetMouseSensitivity _pause_menu_widget)) (Class|Slider|GetValue (Variables|/Game/UI/WBP_PauseMenu1.WBP_PauseMenu1_C|GetGamepadSensitivity _pause_menu_widget)))
        (Input|SetInputModeGameOnly (Game|GetPlayerController 0))
        (Widget|SetVisibility _pause_menu_widget_2 "Collapsed")
        (Widget|SetVisibility (Variables|/Game/UI/WBP_PauseMenu1.WBP_PauseMenu1_C|GetOptionsVb _pause_menu_widget_2) "Collapsed")))))

(event Input|KeyboardEvents|P
  (params (Key :type Key%20Structure :default "None"))
  (bind _pause_menu_widget (Variables|Default|GetPause%20Menu%20Widget))
  (bind _pause_menu_widget_2 (Variables|Default|GetPause%20Menu%20Widget))
  (bind _pause_menu_widget_3 (Variables|Default|GetPause%20Menu%20Widget))
  (:Pressed
    (Utilities|FlowControl|FlipFlop
      (:A
        (Game|SetGamePaused true)
        (Input|SetInputModeGameandUI (Game|GetPlayerController 0) (Variables|Default|GetPause%20Menu%20Widget) "DoNotLock" true)
        (Widget|SetVisibility _pause_menu_widget_3 "Visible")
        (Widget|SetVisibility (Variables|/Game/UI/WBP_PauseMenu1.WBP_PauseMenu1_C|GetMainMenuButtonsVB _pause_menu_widget_3) "Visible")
        (Widget|SetVisibility (Variables|/Game/UI/WBP_PauseMenu1.WBP_PauseMenu1_C|GetMainMenuAllVB _pause_menu_widget_3) "Visible")
        (Variables|/Script/Engine.PlayerController|SetbShowMouseCursor (Game|GetPlayerController 0) true))
      (:B
        (Game|SetGamePaused false)
        (Input|SetInputModeGameOnly (Game|GetPlayerController 0))
        (Widget|SetVisibility _pause_menu_widget_3 "Collapsed")
        (Variables|/Script/Engine.PlayerController|SetbShowMouseCursor (Game|GetPlayerController 0) false)
        (Default|SaveGame _pause_menu_widget (Class|Slider|GetValue (Variables|/Game/UI/WBP_PauseMenu1.WBP_PauseMenu1_C|GetMouseSensitivity _pause_menu_widget)) (Class|Slider|GetValue (Variables|/Game/UI/WBP_PauseMenu1.WBP_PauseMenu1_C|GetGamepadSensitivity _pause_menu_widget)))
        (Input|SetInputModeGameOnly (Game|GetPlayerController 0))
        (Widget|SetVisibility _pause_menu_widget_2 "Collapsed")
        (Widget|SetVisibility (Variables|/Game/UI/WBP_PauseMenu1.WBP_PauseMenu1_C|GetOptionsVb _pause_menu_widget_2) "Collapsed")))))

(event Input|KeyboardEvents|Escape
  (params (Key :type Key%20Structure :default "None"))
  (bind _pause_menu_widget (Variables|Default|GetPause%20Menu%20Widget))
  (bind _pause_menu_widget_2 (Variables|Default|GetPause%20Menu%20Widget))
  (bind _pause_menu_widget_3 (Variables|Default|GetPause%20Menu%20Widget))
  (:Pressed
    (Utilities|FlowControl|FlipFlop
      (:A
        (Game|SetGamePaused true)
        (Input|SetInputModeGameandUI (Game|GetPlayerController 0) (Variables|Default|GetPause%20Menu%20Widget) "DoNotLock" true)
        (Widget|SetVisibility _pause_menu_widget_3 "Visible")
        (Widget|SetVisibility (Variables|/Game/UI/WBP_PauseMenu1.WBP_PauseMenu1_C|GetMainMenuButtonsVB _pause_menu_widget_3) "Visible")
        (Widget|SetVisibility (Variables|/Game/UI/WBP_PauseMenu1.WBP_PauseMenu1_C|GetMainMenuAllVB _pause_menu_widget_3) "Visible")
        (Variables|/Script/Engine.PlayerController|SetbShowMouseCursor (Game|GetPlayerController 0) true))
      (:B
        (Game|SetGamePaused false)
        (Input|SetInputModeGameOnly (Game|GetPlayerController 0))
        (Widget|SetVisibility _pause_menu_widget_3 "Collapsed")
        (Variables|/Script/Engine.PlayerController|SetbShowMouseCursor (Game|GetPlayerController 0) false)
        (Default|SaveGame _pause_menu_widget (Class|Slider|GetValue (Variables|/Game/UI/WBP_PauseMenu1.WBP_PauseMenu1_C|GetMouseSensitivity _pause_menu_widget)) (Class|Slider|GetValue (Variables|/Game/UI/WBP_PauseMenu1.WBP_PauseMenu1_C|GetGamepadSensitivity _pause_menu_widget)))
        (Input|SetInputModeGameOnly (Game|GetPlayerController 0))
        (Widget|SetVisibility _pause_menu_widget_2 "Collapsed")
        (Widget|SetVisibility (Variables|/Game/UI/WBP_PauseMenu1.WBP_PauseMenu1_C|GetOptionsVb _pause_menu_widget_2) "Collapsed")))))

(event Input|GamepadEvents|GamepadFaceButtonRight
  (params (Key :type Key%20Structure :default "None"))
  (bind _pause_menu_widget (Variables|Default|GetPause%20Menu%20Widget))
  (:Pressed
    (if (Widget|IsVisible (Variables|/Game/UI/WBP_PauseMenu1.WBP_PauseMenu1_C|GetOptionsVb _pause_menu_widget))
      (Default|OptionstoMain _pause_menu_widget))))

(event Input|KeyboardEvents|AnyKey
  (params (Key :type Key%20Structure :default "None"))
  (bind _pause_menu_widget (Variables|Default|GetPause%20Menu%20Widget))
  (:Pressed
    (if (not (Class|KismetInputLibrary|KeyIsMouseButton Key))
      (if (Widget|IsVisible (Variables|/Game/UI/WBP_PauseMenu1.WBP_PauseMenu1_C|GetOptionsVb _pause_menu_widget))
        (Widget|SetKeyboardFocus (Variables|/Game/UI/WBP_PauseMenu1.WBP_PauseMenu1_C|GetMouseSensitivity _pause_menu_widget))
        (elif (Widget|IsVisible _pause_menu_widget)
          (Widget|SetKeyboardFocus (Variables|/Game/UI/WBP_PauseMenu1.WBP_PauseMenu1_C|GetResumeGameButton _pause_menu_widget)))))))

(event Input|MouseEvents|LeftMouseButton
  (params (Key :type Key%20Structure :default "None"))
  (:Pressed
    (Class|WidgetBlueprintLibrary|SetFocustoGameViewport)))

(fn ConstructionScript
  (|CallParentFunction))